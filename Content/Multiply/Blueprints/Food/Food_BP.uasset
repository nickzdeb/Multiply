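; Food actor that rots over time and removes itself from the world when its rot countdown runs out.
; On BeginPlay it starts a looping one-second timer that decrements RotTimer and destroys the actor once it is no longer above zero.
; In parallel, the RottingColor timeline drives the Alpha scalar parameter on the mesh materials to show the decay, independently of the countdown.
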(event `self.ReceiveBeginPlay`
  (`KismetSystemLibrary.K2_SetTimer` null "Rotting" 1.0 true)
  (bind (_direction _rot_color_timeline) (`Timeline|Rotting Color`)
    (:`Update`
      (`MeshComponent.SetScalarParameterValueOnMaterials` (`self.Mesh`) "Alpha" _rot_color_timeline))))

(fn `Rotting`
  (if (> (`self.Rot Timer`) 0)
    (`/Engine/EditorBlueprintResources/StandardMacros.DecrementInt` (`self.Rot Timer`))
    (else
      (`self.K2_DestroyActor`))))

(fn `UserConstructionScript`)