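; Creature character with health, hunger and stamina that eats food, melees, sprints, grows up and spawns copies of itself, under player or AI control.
; Looping named timers drive starvation, regeneration, growth, death checks and status bar updates, with lower stat caps for children.
; Growth and non-player hunger and reproduction timers write Blackboard flags for the AI.
; Death ragdolls the body and requests player respawn; damage handling is marked bugged for multiple hits.
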(event `self.ReceiveBeginPlay`
  (`KismetSystemLibrary.K2_SetTimer` null "Starve" 5.0 true)
  (`KismetSystemLibrary.K2_SetTimer` null "Passive Heal" 3.0 true)
  (`KismetSystemLibrary.K2_SetTimer` null "Grow Up" 1.0 true)
  (`KismetSystemLibrary.K2_SetTimer` null "Passive Stamina" 0.5 true)
  (`KismetSystemLibrary.K2_SetTimer` null "Status Update" 0.5 true)
  (bind _ascreature_status_bars (cast `/Game/Multiply/Blueprints/Creatures/Creature/Creature_Status_Bars` (`WidgetComponent.GetWidget` (`self.Status Widget`))))
  (set `self.Status Bar Ref` _ascreature_status_bars)
  (`KismetSystemLibrary.K2_SetTimer` null "Update Status Bars" 0.5 true)
  (if (!= (`self.GetController`) "/Game/Multiply/Blueprints/Player/PlayerController_BP.PlayerController_BP")
    (`KismetSystemLibrary.K2_SetTimer` null "Pregnancy Timer" 1.0 true)
    (`KismetSystemLibrary.K2_SetTimer` null "Is Hungry" 5.0 true)))

(event `self.CapsuleComponent.OnComponentBeginOverlap`
  (params (OverlappedComponent :type "PrimitiveComponent Object Reference") (OtherActor :type "Actor Object Reference") (OtherComp :type "PrimitiveComponent Object Reference") (OtherBodyIndex :type Integer) (bFromSweep :type Boolean) (SweepResult :type "HitResult Structure (by ref)"))
  (bind _hunger (`self.Hunger`))
  (bind _hunger_2 (`self.Hunger`))
  ;[1 1 1] Fill hunger after eating
  (bind _asfood_bp (cast `/Game/Multiply/Blueprints/Food/Food_BP` OtherActor))
  (`self.K2_DestroyActor` _asfood_bp)
  (`self.Add Health`)
  (if (`self.IsGrown`)
    ;[1 1 1] Adult Hunger
    (if (> _hunger_2 100.0)
      (set `self.Hunger` 100.0)
      (else
        (set `self.Hunger` (+ _hunger_2 5.0))))
    (else
      ;[1 1 1] Child Hunger
      (if (> _hunger 75.0)
        (set `self.Hunger` 75.0)
        (else
          (set `self.Hunger` (+ _hunger 7.5)))))))

(event `/Game/Multiply/Blueprints/Combat_INterface.MeleeAttack`
  ;[1 1 1] Punch
  (`|PlayMontage` (`self.Mesh`) "/Game/Multiply/Blueprints/Creatures/Creature/Animations/PunchV6_Montage.PunchV6_Montage"))

(event `self.ReceiveAnyDamage`
  (params (Damage :type "Float (single-precision)") (DamageType :type "DamageType Object Reference") (InstigatedBy :type "Controller Object Reference") (DamageCauser :type "Actor Object Reference"))
  (bind _mesh (`self.Mesh`))
  ;[1 1 1] Damage from hit BUGGED - hits multiple times
  (set `self.Health` (- (`self.Health`) Damage))
  (if (not (`SkeletalMeshComponent.IsPlaying` _mesh))
    (`|PlayMontage` _mesh "/Game/Multiply/Blueprints/Creatures/Creature/Animations/Hit_ReactV1_Montage.Hit_ReactV1_Montage")))

(fn `Add Health`
  (if (`self.IsGrown`)
    ;[1 1 1] Adult Health
    (if (> (`self.Health`) 100.0)
      (set `self.Health` 100.0)
      (elif (< (`self.Health`) 100.0)
        (set `self.Health` (+ (`self.Health`) 5.0))
        (else
          (set `self.Health` 100.0))))
    (else
      ;[1 1 1] Child Health
      (if (> (`self.Health`) 75.0)
        (set `self.Health` 75.0)
        (elif (< (`self.Health`) 75.0)
          (set `self.Health` (+ (`self.Health`) 5.0))
          (else
            (set `self.Health` 75.0)))))))

(fn `Death`
  (bind _returnvalue (`self.GetController` self))
  (`KismetSystemLibrary.K2_ClearTimer` null "Starve")
  (`KismetSystemLibrary.K2_ClearTimer` null "Passive Heal")
  (`KismetSystemLibrary.K2_ClearTimer` null "Grow Up")
  (`KismetSystemLibrary.K2_ClearTimer` null "Passive Stamina")
  (`KismetSystemLibrary.K2_ClearTimer` null "Status Update")
  (`KismetSystemLibrary.K2_ClearTimer` null "Update Status Bars")
  (`|ExecutionSequence`
    (:`then_0`
      (bind _asplayer_controller_bp (cast `/Game/Multiply/Blueprints/Player/PlayerController_BP` _returnvalue))
      (`/Game/Multiply/Blueprints/Player/PlayerController_BP.Respawn` _asplayer_controller_bp self))
    (:`then_1`
      (`Controller.UnPossess` _returnvalue)
      (`PrimitiveComponent.SetSimulatePhysics` (`self.Mesh`) true)
      (`PrimitiveComponent.SetCollisionEnabled` (`self.Mesh`) "PhysicsOnly")
      (`SceneComponent.SetHiddenInGame` (`self.Status Widget`) true false)
      (set `self.IsDead` true))))

(fn `Grow Up`
  (set `self.AgeTimer` (+ (`self.AgeTimer`) 1))
  (if (> (`self.AgeTimer`) 120)
    (`SceneComponent.SetWorldScale3D` (`self.CapsuleComponent`) (0.5 0.5 0.5))
    (set `CharacterMovementComponent.MaxWalkSpeed` 600.0 (`self.CharacterMovement`))
    (`BlackboardComponent.SetValueAsBool` (`AIBlueprintHelperLibrary.GetBlackboard` null) "IsGrown" true)
    (set `self.IsGrown` true)
    (`KismetSystemLibrary.K2_ClearTimer` null "Grow Up")))

(fn `Is Hungry`
  (bind _returnvalue (`AIBlueprintHelperLibrary.GetBlackboard` null))
  (if (<= (`self.Hunger`) 75.0)
    (`/Engine/EditorBlueprintResources/StandardMacros.IsValid` _returnvalue
      (:`Is Valid`
        (`BlackboardComponent.SetValueAsBool` _returnvalue "IsHungry" true)))))

(fn `Passive Heal`
  (if (`self.IsGrown`)
    ;[1 1 1] Adult Health
    (if (> (`self.Health`) 100.0)
      (set `self.Health` 100.0)
      (elif (< (`self.Health`) 100.0)
        (set `self.Health` (+ (`self.Health`) 2.5))
        (else
          (set `self.Health` 100.0))))
    (else
      ;[1 1 1] Child Health
      (if (> (`self.Health`) 75.0)
        (set `self.Health` 75.0)
        (elif (< (`self.Health`) 75.0)
          (set `self.Health` (+ (`self.Health`) 2.5))
          (else
            (set `self.Health` 75.0)))))))

(fn `Passive Stamina`
  (if (`self.IsGrown`)
    ;[1 1 1] Adult Stamina
    (if (> (`self.Stamina`) 100.0)
      (set `self.Stamina` 100.0)
      (elif (< (`self.Stamina`) 100.0)
        (set `self.Stamina` (+ (`self.Stamina`) 2.5))
        (else
          (set `self.Stamina` 100.0))))
    (else
      ;[1 1 1] Child Stamina
      (if (> (`self.Stamina`) 75.0)
        (set `self.Stamina` 75.0)
        (elif (< (`self.Stamina`) 75.0)
          (set `self.Stamina` (+ (`self.Stamina`) 1.5))
          (else
            (set `self.Stamina` 75.0)))))))

(fn `Pregnancy Timer`
  (bind _returnvalue (`AIBlueprintHelperLibrary.GetBlackboard` null))
  (bind _output_get (set `self.MultiplyTimer` (- (`self.MultiplyTimer`) 1)))
  (if (<= _output_get 0)
    (`/Engine/EditorBlueprintResources/StandardMacros.IsValid` _returnvalue
      (:`Is Valid`
        (`BlackboardComponent.SetValueAsBool` _returnvalue "AbleToReproduce" true)))
    (else
      (`/Engine/EditorBlueprintResources/StandardMacros.IsValid` _returnvalue
        (:`Is Valid`
          (`BlackboardComponent.SetValueAsBool` _returnvalue "AbleToReproduce" false))))))

(fn `Reproduce`
  (if (and (> (`self.Hunger`) 75.0) (> (`self.Stamina`) 75.0) (`self.IsGrown`))
    (`|SpawnActorFromClass` (`GameplayStatics.GetObjectClass` self) (`KismetMathLibrary.MakeTransform` (`self.K2_GetActorLocation` self)) "AdjustIfPossibleButAlwaysSpawn" "OverrideRootScale" null null)
    (set `self.Hunger` (- (`self.Hunger`) 50.0))
    (set `self.Stamina` 0.0)
    (set `self.MultiplyTimer` 120)))

(fn `Spend Stamina`
  (if (> (`self.Stamina`) 0.0)
    (if (> (`KismetMathLibrary.VSize` (`self.GetVelocity` self)) 400.0)
      (set `self.Stamina` (- (`self.Stamina`) 1.0)))
    (else
      (set `self.Stamina` 0.0)
      (`self.unSprint`))))

(fn `Sprint`
  (if (> (`self.Stamina`) 0.0)
    (set `CharacterMovementComponent.MaxWalkSpeed` 650.0 (`self.CharacterMovement`))
    (`KismetSystemLibrary.K2_SetTimer` null "Spend Stamina" 0.2 true)
    (`KismetSystemLibrary.K2_ClearTimer` null "Passive Stamina")))

(fn `Starve`
  (set `self.Hunger` (- (`self.Hunger`) 2.0)))

(fn `Status Update`
  (`|ExecutionSequence`
    (:`then_0`
      (if (<= (`self.Hunger`) 0.0)
        (`self.Death`)))
    (:`then_1`
      (if (<= (`self.Health`) 0.0)
        (`self.Death`)))))

(fn `unSprint`
  (set `CharacterMovementComponent.MaxWalkSpeed` 400.0 (`self.CharacterMovement`))
  (`KismetSystemLibrary.K2_ClearTimer` null "Spend Stamina")
  (`KismetSystemLibrary.K2_SetTimer` null "Passive Stamina" 0.5 true))

(fn `Update Status Bars`
  (bind _stamina (`self.Stamina`))
  (bind _health (`self.Health`))
  (bind _hunger (`self.Hunger`))
  (bind _healthbar (`/Game/Multiply/Blueprints/Creatures/Creature/Creature_Status_Bars.HealthBar` (`self.Status Bar Ref`)))
  (bind _hungerbar (`/Game/Multiply/Blueprints/Creatures/Creature/Creature_Status_Bars.HungerBar` (`self.Status Bar Ref`)))
  (bind _staminabar (`/Game/Multiply/Blueprints/Creatures/Creature/Creature_Status_Bars.StaminaBar` (`self.Status Bar Ref`)))
  (`|ExecutionSequence`
    (:`then_0`
      (if (`self.IsGrown`)
        (`ProgressBar.SetPercent` _healthbar (/ _health 100.0))
        (else
          (`ProgressBar.SetPercent` _healthbar (/ (* _health 1.333) 100.0)))))
    (:`then_1`
      (if (`self.IsGrown`)
        (`ProgressBar.SetPercent` _hungerbar (/ _hunger 100.0))
        (else
          (`ProgressBar.SetPercent` _hungerbar (/ (* _hunger 1.333) 100.0)))))
    (:`then_2`
      (if (`self.IsGrown`)
        (`ProgressBar.SetPercent` _staminabar (/ _stamina 100.0))
        (else
          (`ProgressBar.SetPercent` _staminabar (/ (* _stamina 1.333) 100.0)))))))

(fn `UserConstructionScript`)